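; Start menu controller actor that drives the UI flow from the main menu through three story screens and into Level1.
; BeginPlay shows the main menu, and each GoTo function clears all widgets, then creates and displays its story screen.
; Every created widget receives a reference to this controller, allowing it to call the navigation functions.
; LoadLevel1 clears the UI and loads Level1 as a level instance.
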(event EventBeginPlay
  (bind _returnvalue (UserInterface|CreateWidget "/Game/Blueprints/StartMenu/MainMenuWidget.MainMenuWidget_C"))
  (bind _output_get (Variables|Default|SetMainMenu _returnvalue))
  (Variables|/Game/Blueprints/StartMenu/MainMenuWidget.MainMenuWidget_C|SetWidgetController _output_get self)
  (UserInterface|Viewport|AddtoViewport _output_get 0))

(event Collision|EventActorBeginOverlap
  (params (OtherActor :type Actor%20Object%20Reference)))

(event EventTick
  (params (DeltaSeconds :type Float%20%28single-precision%29)))

(fn ConstructionScript)

(fn ClearWidgets
  (Viewport|RemoveAllWidgets))

(fn GotoStory1
  (CallFunction|ClearWidgets)
  (bind _returnvalue (UserInterface|CreateWidget "/Game/Blueprints/StartMenu/Story1.Story1_C"))
  (bind _output_get (Variables|Default|SetStory1 _returnvalue))
  (Variables|/Game/Blueprints/StartMenu/Story1.Story1_C|SetWidgetController _output_get self)
  (UserInterface|Viewport|AddtoViewport _output_get 0))

(fn GotoStory2
  (CallFunction|ClearWidgets)
  (bind _returnvalue (UserInterface|CreateWidget "/Game/Blueprints/StartMenu/Story2.Story2_C"))
  (bind _output_get (Variables|Default|SetStory2 _returnvalue))
  (Variables|/Game/Blueprints/StartMenu/Story2.Story2_C|SetWidgetController _output_get self)
  (UserInterface|Viewport|AddtoViewport _output_get 0))

(fn GotoStory3
  (CallFunction|ClearWidgets)
  (bind _returnvalue (UserInterface|CreateWidget "/Game/Blueprints/StartMenu/Story3.Story3_C"))
  (bind _output_get (Variables|Default|SetStory3 _returnvalue))
  (Variables|/Game/Blueprints/StartMenu/Story3.Story3_C|SetWidgetController _output_get self)
  (UserInterface|Viewport|AddtoViewport _output_get 0))

(fn LoadLevel1
  (CallFunction|ClearWidgets)
  (Class|LevelStreamingDynamic|LoadLevelInstance "Level1" "0, 0, 0" "0, 0, 0"))