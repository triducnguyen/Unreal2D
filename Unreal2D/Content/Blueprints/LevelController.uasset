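; LevelController is an actor that manages spawn points and level transitions in a 2D side-scroller.
; It caches the 2DSideScrollerGameMode during construction and again on BeginPlay, then sets its SpawnTransform from the Start actor.
; SetSpawn overwrites that transform and prints a confirmation.
; EndLevel clears the exit key flag, destroys the player pawn and loads NextLevel as a level instance.
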(event EventBeginPlay
  (bind _as2dside_scroller_game_mode (Utilities|Casting|CastTo2DSideScrollerGameMode (Game|GetGameMode)))
  (bind _output_get (Variables|Default|SetGameMode _as2dside_scroller_game_mode))
  (Variables|/Game/2DSideScrollerBP/Blueprints/2DSideScrollerGameMode.2DSideScrollerGameMode_C|SetSpawn%20Transform _output_get (Transformation|GetActorTransform (Variables|Default|GetStart))))

(event Collision|EventActorBeginOverlap
  (params (OtherActor :type Actor%20Object%20Reference)))

(event EventTick
  (params (DeltaSeconds :type Float%20%28single-precision%29)))

(fn ConstructionScript
  (bind _as2dside_scroller_game_mode (Utilities|Casting|CastTo2DSideScrollerGameMode (Game|GetGameMode)))
  (Variables|Default|SetGameMode _as2dside_scroller_game_mode))

(fn EndLevel
  (Variables|Default|SetHasExitKey false)
  (Actor|DestroyActor (Game|Player|GetPlayerPawn 0))
  (Class|LevelStreamingDynamic|LoadLevelInstance (Variables|Default|GetNextLevel) "0, 0, 0" "0, 0, 0"))

(fn SetSpawn
  (params (NewSpawn :type Transform))
  (Variables|/Game/2DSideScrollerBP/Blueprints/2DSideScrollerGameMode.2DSideScrollerGameMode_C|SetSpawn%20Transform (Variables|Default|GetGameMode) NewSpawn)
  (Development|PrintString "Set new spawn"))